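; Inventory component that stores items in a fixed number of slots, created empty on BeginPlay.
; AddItem places units one at a time, filling matching stacks before empty slots, and returns the count that did not fit.
; MoveItems works within or across inventories, merging same-item stacks with overflow left in the source, swapping different items or filling empty slots.
; Helpers decrement slots and spawn dropped items at an owner-supplied position.
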(event `self.ReceiveBeginPlay`
  (`self.InitializeInventory`))

(fn `AddItem`
  (params (ItemToAdd :type "/Game/_Main/Data/Items/PDA_Items Object Reference") (QuantityToAdd :type Integer))
  (returns (ItemsLeft :type Integer))
  (locals (ItemsLeftToAdd :type Integer))
  (set `local.ItemsLeftToAdd` QuantityToAdd)
  (for _ (range 1 (+ QuantityToAdd 1))
    (if (`/Game/_Main/Data/Items/PDA_Items.IsStackable` ItemToAdd)
      (bind (_success _slotindex) (`self.FindAvailableStackableSlot` (`local.ItemToAdd`)))
      (if _success
        (`self.AddItemToStackableSlot` _slotindex)
        (set `local.ItemsLeftToAdd` (- (`local.ItemsLeftToAdd`) 1))
        (else
          (bind (_success_2 _slotindex_2) (`self.FindEmptySlot` :!label _label))
          (if _success_2
            (`self.AddItemToEmptySlot` _slotindex_2 (`local.ItemToAdd`))
            (set `local.ItemsLeftToAdd` (- (`local.ItemsLeftToAdd`) 1))
            (else
              (`KismetSystemLibrary.PrintString` "Inventory Full")))))
      (else
        (goto _label))))
  (return (`local.ItemsLeftToAdd`)))

(fn `AddItemToEmptySlot`
  (params (SlotIndex :type Integer) (ItemToAdd :type "/Game/_Main/Data/Items/PDA_Items Object Reference"))
  (`KismetArrayLibrary.Array_Set` (`self.InventorySlots`) SlotIndex (make `/Game/_Main/Data/Inventory/S_InventorySlot` ItemToAdd 1 true))
  (return))

(fn `AddItemToStackableSlot`
  (params (SlotIndex :type Integer))
  (bind _output (`|GetArrayItem` (`self.InventorySlots`) SlotIndex))
  (setmembers `/Game/_Main/Data/Inventory/S_InventorySlot` :`StructRef` _output :`Quantity` (+ (`.Quantity_9_E54807A14508C6CD21DF009F3C4A289C` (break `/Game/_Main/Data/Inventory/S_InventorySlot` _output)) 1))
  (return))

(fn `DecrementSlotQuantity`
  (params (SlotIndex :type Integer) (QuantityToDecrement :type Integer))
  (bind _output (`|GetArrayItem` (`self.InventorySlots`) SlotIndex))
  (bind _returnvalue (- (`.Quantity_9_E54807A14508C6CD21DF009F3C4A289C` (break `/Game/_Main/Data/Inventory/S_InventorySlot` _output)) QuantityToDecrement))
  (if (<= _returnvalue 0)
    (`KismetArrayLibrary.Array_Set` (`self.InventorySlots`) SlotIndex (make `/Game/_Main/Data/Inventory/S_InventorySlot` null))
    (else
      (setmembers `/Game/_Main/Data/Inventory/S_InventorySlot` :`StructRef` _output :`Quantity` _returnvalue))))

(fn `FindAvailableStackableSlot`
  (params (ItemToAdd :type "/Game/_Main/Data/Items/PDA_Items Object Reference"))
  (returns (Success :type Boolean) (SlotIndex :type Integer))
  (for (_array_element _array_index) (`self.InventorySlots`)
    (bind ((`ItemData_14_9E7E26F74402034797E9E3AE85FE97E2` _itemdata) (`Quantity_9_E54807A14508C6CD21DF009F3C4A289C` _quantity)) (break `/Game/_Main/Data/Inventory/S_InventorySlot` _array_element))
    (if (and (== (`local.ItemToAdd`) _itemdata) (<= (+ _quantity 1) (`/Game/_Main/Data/Items/PDA_Items.MaxStackSize` ItemToAdd)))
      (return true _array_index)))
  (return false -1))

(fn `FindEmptySlot`
  (returns (Success :type Boolean) (SlotIndex :type Integer))
  (for (_array_element _array_index) (`self.InventorySlots`)
    (if (not (`.IsOccupied_8_D033D983469E21FBF200CABE2E9FABEC` (break `/Game/_Main/Data/Inventory/S_InventorySlot` _array_element)))
      (return true _array_index)))
  (return false -1))

(fn `IncreaseStack`
  (params (TargetSlotIndex :type Integer) (QuantityToAdd :type Integer))
  (returns (QuantityLeft :type Integer))
  (locals (TargetSlot :type "/Game/_Main/Data/Inventory/S_InventorySlot Structure") (ItemData :type "/Game/_Main/Data/Items/PDA_Items Object Reference"))
  (bind _maxstacksize (`/Game/_Main/Data/Items/PDA_Items.MaxStackSize` (`local.ItemData`)))
  (bind _returnvalue (+ (`.Quantity_9_E54807A14508C6CD21DF009F3C4A289C` (break `/Game/_Main/Data/Inventory/S_InventorySlot` (`local.TargetSlot`))) (`local.QuantityToAdd`)))
  (`|ExecutionSequence`
    (:`then_0`
      (bind _output_get (set `local.TargetSlot` (`|GetArrayItem` (`self.InventorySlots`) TargetSlotIndex)))
      (set `local.ItemData` (`.ItemData_14_9E7E26F74402034797E9E3AE85FE97E2` (break `/Game/_Main/Data/Inventory/S_InventorySlot` _output_get))))
    (:`then_1`
      (if (> _returnvalue (`/Game/_Main/Data/Items/PDA_Items.MaxStackSize` (`local.ItemData`)))
        (setmembers `/Game/_Main/Data/Inventory/S_InventorySlot` :`StructRef` (`|GetArrayItem` (`self.InventorySlots`) (`local.TargetSlotIndex`)) :`Quantity` _maxstacksize)
        (return (- (+ (`.Quantity_9_E54807A14508C6CD21DF009F3C4A289C` (break `/Game/_Main/Data/Inventory/S_InventorySlot` (`local.TargetSlot`))) (`local.QuantityToAdd`)) _maxstacksize))
        (else
          (setmembers `/Game/_Main/Data/Inventory/S_InventorySlot` :`StructRef` (`|GetArrayItem` (`self.InventorySlots`) (`local.TargetSlotIndex`)) :`Quantity` _returnvalue)
          (return 0))))))

(fn `InitializeInventory`
  (for _ (range 1 (+ (`self.SlotsCount`) 1))
    (`KismetArrayLibrary.Array_Add` (`self.InventorySlots`) (make `/Game/_Main/Data/Inventory/S_InventorySlot` null))))

(fn `MoveItems`
  (params (SourceInventory :type "/Game/_Main/Data/Inventory/BPC_Inventory Object Reference") (SourceSlotIndex :type Integer) (TargetSlotIndex :type Integer))
  (locals (SourceSlot :type "/Game/_Main/Data/Inventory/S_InventorySlot Structure") (TargetSlot :type "/Game/_Main/Data/Inventory/S_InventorySlot Structure"))
  (bind (_itemdata _quantity _isoccupied) (break `/Game/_Main/Data/Inventory/S_InventorySlot` (`local.SourceSlot`)))
  (bind ((`ItemData_14_9E7E26F74402034797E9E3AE85FE97E2` _itemdata_2) (`Quantity_9_E54807A14508C6CD21DF009F3C4A289C` _quantity_2)) (break `/Game/_Main/Data/Inventory/S_InventorySlot` (`local.SourceSlot`)))
  (set `local.SourceSlot` (`|GetArrayItem` (`/Game/_Main/Data/Inventory/BPC_Inventory.InventorySlots` SourceInventory) SourceSlotIndex))
  (bind _output_get (set `local.TargetSlot` (`|GetArrayItem` (`self.InventorySlots`) TargetSlotIndex)))
  (if (`.IsOccupied_8_D033D983469E21FBF200CABE2E9FABEC` (break `/Game/_Main/Data/Inventory/S_InventorySlot` _output_get))
    (if (== _itemdata_2 (`.ItemData_14_9E7E26F74402034797E9E3AE85FE97E2` (break `/Game/_Main/Data/Inventory/S_InventorySlot` (`local.TargetSlot`))))
      (bind _quantityleft (`self.IncreaseStack` (`local.TargetSlotIndex`) _quantity_2))
      (if (> _quantityleft 0)
        (setmembers `/Game/_Main/Data/Inventory/S_InventorySlot` :`StructRef` (`|GetArrayItem` (`/Game/_Main/Data/Inventory/BPC_Inventory.InventorySlots` (`local.SourceInventory`)) (`local.SourceSlotIndex`)) :`Quantity` _quantityleft)
        (else
          (setmembers `/Game/_Main/Data/Inventory/S_InventorySlot` :`StructRef` (`|GetArrayItem` (`/Game/_Main/Data/Inventory/BPC_Inventory.InventorySlots` (`local.SourceInventory`)) (`local.SourceSlotIndex`)) :`ItemData` null :`Quantity` 0 :`IsOccupied` false :!label _label)))
      (else
        (`KismetArrayLibrary.Array_Set` (`/Game/_Main/Data/Inventory/BPC_Inventory.InventorySlots` (`local.SourceInventory`)) (`local.SourceSlotIndex`) (`local.TargetSlot`))
        (`KismetArrayLibrary.Array_Set` (`self.InventorySlots`) (`local.TargetSlotIndex`) (`local.SourceSlot`))))
    (else
      (setmembers `/Game/_Main/Data/Inventory/S_InventorySlot` :`StructRef` (`|GetArrayItem` (`self.InventorySlots`) (`local.TargetSlotIndex`)) :`ItemData` _itemdata :`Quantity` _quantity :`IsOccupied` _isoccupied)
      (goto _label))))

(fn `SpawnDroppedItems`
  (bind _itemtospawn (`self.ItemToSpawn`)
    (:`then`
      (bind _dropposition (message `/Game/_Main/Interfaces/BPI_Player.GetDropPosition` (`self.GetOwner`)))
      (`|SpawnActorFromClass` _itemtospawn (`KismetMathLibrary.MakeTransform` _dropposition) "Undefined" "MultiplyWithRoot" null null))
    (:`else`)))