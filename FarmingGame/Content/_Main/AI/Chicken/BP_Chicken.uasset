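; BP_Chicken is a chicken actor that periodically lays eggs.
; From BeginPlay, a looping Delay of random length spawns a BP_Egg at the root component's location, giving each egg a random Quantity.
; A separate PlaySound event plays the chicken death sound at that same location.
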(event `self.ReceiveBeginPlay`
  (`KismetSystemLibrary.Delay` (`KismetMathLibrary.RandomFloatInRange` 30.0 120.0) :!label _label)
  (`|SpawnActorFromClass` "/Game/_Main/Blueprints/Collectables/BP_Egg.BP_Egg_C" (`KismetMathLibrary.MakeTransform` (`SceneComponent.K2_GetComponentLocation` (`self.DefaultSceneRoot`))) "Undefined" "MultiplyWithRoot" null (`KismetMathLibrary.RandomIntegerInRange` 1 4) null)
  (goto _label))

(event `/Game/_Main/Data/Interfaces/BPI_Animals.PlaySound`
  (`GameplayStatics.PlaySoundAtLocation` "/Game/_Main/Sounds/ChickenDie.ChickenDie" (`SceneComponent.K2_GetComponentLocation` (`self.DefaultSceneRoot`)) (struct) 1.0 1.0 0.0 null null null null))

(fn `UserConstructionScript`
  (`parent.UserConstructionScript`))