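; Animal actor that takes hits, dies and yields item drops.
; Each TakeDamage call removes one Health point; at zero or below it plays a montage on its skeletal mesh.
; When the montage completes, it sends player character 0 a message to spawn a random small count of its ItemData item, then destroys itself.
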(event `/Game/_Main/Data/Interfaces/BPI_Animals.TakeDamage`
  (bind _output_get (set `self.Health` (- (`self.Health`) 1)))
  (if (<= _output_get 0)
    (`|PlayMontage` (`self.SkeletalMesh`) (`self.Montage`)
      (:`OnCompleted`
        (message `/Game/_Main/Data/Interfaces/BPI_Player.SpawnDroppedItems` (`GameplayStatics.GetPlayerCharacter` 0) (`KismetMathLibrary.RandomIntegerInRange` 1 3) (`self.ItemData`))
        (`self.K2_DestroyActor`)))))

(fn `UserConstructionScript`)