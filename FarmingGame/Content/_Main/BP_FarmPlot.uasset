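; BP_FarmPlot is an interactable farm plot that grows wheat and is cleared once grown.
; Interacting in the initial state starts a timed Delay chain that swaps the Socket mesh from seeds through three wheat sizes.
; A PlotStates enum tracks progress, and CanInteract allows use only in the initial or fully grown state.
; Interact itself resets any non-initial plot without checking growth.
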(event `/Game/_Main/Interfaces/BPI_Interactable.Interact`
  (if (`|EnumEquality` (`self.PlotStates`) "NewEnumerator0")
    (set `self.PlotStates` "NewEnumerator1")
    (`StaticMeshComponent.SetStaticMesh` (`self.Socket`) "/Game/_Main/Meshes/Seeds.Seeds")
    (`KismetSystemLibrary.Delay` 5.0)
    (`StaticMeshComponent.SetStaticMesh` (`self.Socket`) "/Game/_Main/Meshes/WheatSmall.WheatSmall")
    (`KismetSystemLibrary.Delay` 5.0)
    (`StaticMeshComponent.SetStaticMesh` (`self.Socket`) "/Game/_Main/Meshes/WheatMedium.WheatMedium")
    (`KismetSystemLibrary.Delay` 5.0)
    (`StaticMeshComponent.SetStaticMesh` (`self.Socket`) "/Game/_Main/Meshes/WheatBig.WheatBig")
    (set `self.PlotStates` "NewEnumerator4")
    (else
      (set `self.PlotStates` "NewEnumerator0")
      (`StaticMeshComponent.SetStaticMesh` (`self.Socket`) null))))

(fn `CanInteract`
  (returns (State :type Boolean))
  (bind _plotstates (`self.PlotStates`))
  (return (or (`|EnumEquality` _plotstates "NewEnumerator0") (`|EnumEquality` _plotstates "NewEnumerator4"))))

(fn `UserConstructionScript`)