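; BP_Plant is an interactable plant that may give seeds when harvested.
; On BeginPlay it picks a random seed entry and rolls a quantity from a range reaching below zero, so many plants yield nothing.
; On Interact it sends any positive yield to the instigator's inventory by message calls, passes the leftover count to be spawned as dropped items, then destroys itself.
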(event `self.ReceiveBeginPlay`
  (`parent.ReceiveBeginPlay`)
  (set `self.DropData` (`|GetArrayItem` (`self.SeedsData`) (`KismetMathLibrary.RandomIntegerInRange` 0 (`KismetArrayLibrary.Array_LastIndex` (`self.SeedsData`)))))
  (set `self.DropQuantity` (`KismetMathLibrary.RandomIntegerInRange` -5 3)))

(event `/Game/_Main/Data/Interfaces/BPI_Interactable.Interact`
  (params (Instigator :type "Actor Object Reference"))
  (bind _dropdata (`self.DropData`))
  (`|ExecutionSequence`
    (:`then_0`
      (if (> (`self.DropQuantity`) 0)
        (bind _itemsleft (message `/Game/_Main/Data/Interfaces/BPI_Player.AddItemToInventory` Instigator _dropdata (`self.DropQuantity`)))
        (message `/Game/_Main/Data/Interfaces/BPI_Player.SpawnDroppedItems` Instigator _itemsleft _dropdata)))
    (:`then_1`
      (`self.K2_DestroyActor`))))

(fn `UserConstructionScript`
  (`parent.UserConstructionScript`))