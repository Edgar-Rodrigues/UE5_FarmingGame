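; BP_BuySign is an interactable sign that lets the player buy an actor in its place.
; On Interact, it reads the instigator's money through interface messages and, if that covers Cost, deducts the amount.
; It then spawns ActorToSpawn at its own transform, ignoring collisions, and destroys itself, making it a one-time purchase.
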(event `/Game/_Main/Data/Interfaces/BPI_Interactable.Interact`
  (params (Instigator :type "Actor Object Reference"))
  (bind _cost (`self.Cost`))
  (bind _money (message `/Game/_Main/Data/Interfaces/BPI_Player.GetMoney` Instigator))
  (if (>= _money _cost)
    (message `/Game/_Main/Data/Interfaces/BPI_Player.SetMoney` Instigator (- _money _cost))
    (`|SpawnActorFromClass` (`self.ActorToSpawn`) (`self.GetTransform`) "AlwaysSpawn" "MultiplyWithRoot" null null)
    (`self.K2_DestroyActor`)))

(fn `UserConstructionScript`
  (`parent.UserConstructionScript`))