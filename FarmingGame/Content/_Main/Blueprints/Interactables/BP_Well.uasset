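; BP_Well is an interactable well that gives its instigator one unit of its item per interaction while stock remains.
; Stock starts at the maximum on BeginPlay, and each Interact sends an add-to-inventory message, then decrements the count.
; Tick refills one unit at a time through a one-minute Delay whenever stock is below the maximum, relying on the pending Delay to throttle repeated ticks.
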(event `self.ReceiveBeginPlay`
  (`parent.ReceiveBeginPlay`)
  (set `self.CurrentQuantity` (`self.MaxQuantity`)))

(event `self.ReceiveTick`
  (params (DeltaSeconds :type "Float (single-precision)"))
  (`parent.ReceiveTick` DeltaSeconds)
  (if (< (`self.CurrentQuantity`) (`self.MaxQuantity`))
    (`KismetSystemLibrary.Delay` 60.0)
    (set `self.CurrentQuantity` (+ (`self.CurrentQuantity`) 1))))

(event `/Game/_Main/Data/Interfaces/BPI_Interactable.Interact`
  (params (Instigator :type "Actor Object Reference"))
  (if (> (`self.CurrentQuantity`) 0)
    (message `/Game/_Main/Data/Interfaces/BPI_Player.AddItemToInventory` Instigator (`self.ItemData`) 1)
    (set `self.CurrentQuantity` (- (`self.CurrentQuantity`) 1))))

(fn `UserConstructionScript`
  (`parent.UserConstructionScript`))