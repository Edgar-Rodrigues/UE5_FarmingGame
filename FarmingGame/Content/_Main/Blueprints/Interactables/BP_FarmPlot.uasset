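; BP_FarmPlot is an interactable plot where the player plants seeds and harvests the grown crop.
; Interacting while empty takes a seed from the instigator's selected hotbar slot, stores its data asset and disables interaction during growth.
; A Delay loop steps through that asset's timed growth-stage meshes, then re-enables interaction.
; Harvesting clears the mesh and grants random drop quantities, passing leftovers to be spawned as dropped items.
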(event `/Game/_Main/Data/Interfaces/BPI_Interactable.Interact`
  (params (Instigator :type "Actor Object Reference"))
  (bind _returnvalue (`self.GetComponentByClass` Instigator "/Game/_Main/Data/Inventory/BPC_Inventory.BPC_Inventory_C"))
  (bind _growthstageindex (`self.GrowthStageIndex`))
  (bind (_staticmesh _time) (break `/Game/_Main/Data/Items/Seeds/S_GrowthStage` (`|GetArrayItem` (`/Game/_Main/Data/Items/Seeds/PDA_Items_Seeds.GrowthStages` (`self.ItemData`)) _growthstageindex)))
  (if (`|EnumEquality` (`self.PlotStates`) "NewEnumerator0")
    (bind _slotindex (message `/Game/_Main/Data/Interfaces/BPI_Player.GetCurrentHotbarSlotIndex` Instigator))
    (bind ((`ItemData_14_9E7E26F74402034797E9E3AE85FE97E2` _itemdata)) (break `/Game/_Main/Data/Inventory/S_InventorySlot` (`|GetArrayItem` (`/Game/_Main/Data/Inventory/BPC_Inventory.InventorySlots` _returnvalue) _slotindex)))
    (if (`GameplayStatics.ObjectIsA` _itemdata "/Game/_Main/Data/Items/Seeds/PDA_Items_Seeds.PDA_Items_Seeds_C")
      (`|ExecutionSequence`
        (:`then_0`
          (bind _aspda_items_seeds (cast `/Game/_Main/Data/Items/Seeds/PDA_Items_Seeds` _itemdata))
          (set `self.ItemData` _aspda_items_seeds)
          (`GameplayStatics.PlaySoundAtLocation` "/Game/_Main/Sounds/PlantSeeds.PlantSeeds" (`SceneComponent.K2_GetComponentLocation` (`self.DefaultSceneRoot`)) (struct) 1.0 1.0 0.0 null null null null))
        (:`then_1`
          (set `self.CanInteractState` false)
          (`/Game/_Main/Data/Inventory/BPC_Inventory.DecrementSlotQuantity` _returnvalue _slotindex 1))
        (:`then_2`
          (set `self.PlotStates` "NewEnumerator1")
          (`StaticMeshComponent.SetStaticMesh` (`self.CropSocket`) _staticmesh :!label _label)
          (`KismetSystemLibrary.Delay` _time)
          (if (== _growthstageindex (- (`KismetArrayLibrary.Array_Length` (`/Game/_Main/Data/Items/Seeds/PDA_Items_Seeds.GrowthStages` (`self.ItemData`))) 1))
            (set `self.PlotStates` "NewEnumerator4")
            (set `self.GrowthStageIndex` 0)
            (set `self.CanInteractState` true)
            (else
              (set `self.GrowthStageIndex` (+ (`self.GrowthStageIndex`) 1))
              (goto _label))))))
    (else
      (set `self.PlotStates` "NewEnumerator0")
      (`StaticMeshComponent.SetStaticMesh` (`self.CropSocket`) null)
      (for _array_element (`/Game/_Main/Data/Items/Seeds/PDA_Items_Seeds.Drops` (`self.ItemData`))
        (bind (_itemdata_2 _minquantity _maxquantity) (break `/Game/_Main/Data/Items/Seeds/S_Drops` _array_element))
        (bind _itemsleft (message `/Game/_Main/Data/Interfaces/BPI_Player.AddItemToInventory` Instigator _itemdata_2 (`KismetMathLibrary.RandomIntegerInRange` _minquantity _maxquantity)))
        (message `/Game/_Main/Data/Interfaces/BPI_Player.SpawnDroppedItems` Instigator _itemsleft _itemdata_2)
        (`GameplayStatics.PlaySoundAtLocation` "/Game/_Main/Sounds/HarvestPlant.HarvestPlant" (`SceneComponent.K2_GetComponentLocation` (`self.DefaultSceneRoot`)) (struct) 1.0 1.0 0.0 null null null null)))))

(fn `UserConstructionScript`
  (`parent.UserConstructionScript`))