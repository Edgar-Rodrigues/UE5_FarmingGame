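; BPM_Collectable is a pickup actor that gives its item to the inventory of whoever interacts with it.
; On Interact it plays a pickup sound and passes ItemData and Quantity to the instigator through an AddItemToInventory interface message.
; The returned value becomes the remaining Quantity, and the actor is destroyed when that value is zero.
; An optional Lifespan flag removes it automatically after a fixed time from BeginPlay.
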(event `self.ReceiveBeginPlay`
  (`parent.ReceiveBeginPlay`)
  (if (`self.Lifespan`)
    (`self.SetLifeSpan` 300.0)))

(event `/Game/_Main/Data/Interfaces/BPI_Interactable.Interact`
  (params (Instigator :type "Actor Object Reference"))
  (`GameplayStatics.PlaySoundAtLocation` "/Game/_Main/Sounds/PickupItem.PickupItem" (`SceneComponent.K2_GetComponentLocation` (`self.DefaultSceneRoot`)) (struct) 1.0 1.0 0.0 null null null null)
  (bind _itemsleft (message `/Game/_Main/Data/Interfaces/BPI_Player.AddItemToInventory` Instigator (`self.ItemData`) (`self.Quantity`)))
  (if (== _itemsleft 0)
    (`self.K2_DestroyActor`)
    (else
      (set `self.Quantity` _itemsleft))))

(fn `UserConstructionScript`
  (`parent.UserConstructionScript`))